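; CarRemover is a valet-game actor that sends the requested car away once it has been dropped off in the pickup zone.
; When a CarPawn enters PickupZone with the ID the ValetGameMode wants retrieved, it binds RemoveCar to that car's exit event.
; RemoveCar spawns the car's default controller and uses SimpleMoveToLocation to send it to KillTransform.
; Leaving the zone unbinds the event.
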(event `self.PickupZone.OnComponentBeginOverlap`
  (params (OverlappedComponent :type "PrimitiveComponent Object Reference") (OtherActor :type "Actor Object Reference") (OtherComp :type "PrimitiveComponent Object Reference") (OtherBodyIndex :type Integer) (bFromSweep :type Boolean) (SweepResult :type "HitResult Structure (by ref)"))
  (bind _ascar_pawn (cast `/Game/Blueprints/CarPawn` OtherActor))
  (bind _id (`/Game/Blueprints/CarPawn.GetCarID` _ascar_pawn))
  (if (== (`/Game/Blueprints/ValetGameMode.CarIDToRetrieve` (cast `/Game/Blueprints/ValetGameMode` (`GameplayStatics.GetGameMode`) :!pure true)) _id)
    (add `/Game/Blueprints/CarPawn.CarExited` _ascar_pawn (delegate `RemoveCar`))))

(event `RemoveCar`
  (`Pawn.SpawnDefaultController` (stale `self.PickupZone.OnComponentBeginOverlap` _ascar_pawn))
  (`AIBlueprintHelperLibrary.SimpleMoveToLocation` (`Pawn.GetController` (stale `self.PickupZone.OnComponentBeginOverlap` _ascar_pawn)) (`SceneComponent.K2_GetComponentLocation` (`self.KillTransform`))))

(event `self.PickupZone.OnComponentEndOverlap`
  (params (OverlappedComponent :type "PrimitiveComponent Object Reference") (OtherActor :type "Actor Object Reference") (OtherComp :type "PrimitiveComponent Object Reference") (OtherBodyIndex :type Integer))
  (bind _ascar_pawn (cast `/Game/Blueprints/CarPawn` OtherActor))
  (remove `/Game/Blueprints/CarPawn.CarExited` _ascar_pawn (delegate `RemoveCar`)))

(fn `UserConstructionScript`)