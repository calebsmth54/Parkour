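; CarPawn is a drivable car for a valet game that gets a random paint and registers with ValetGameMode on spawn.
; Input axes push the physics mesh with forces and rotate it, with turning locked unless world X velocity exceeds a small threshold.
; Interact spawns and possesses a ValetPawn beside the car, reporting it parked if inside a parking zone.
; Possession changes drive engine sounds and FloatingPawnMovement activation.
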(event `self.ReceiveBeginPlay`
  (bind _paints (`self.Paints`))
  (`MovementComponent.SetUpdatedComponent` (`self.FloatingPawnMovement`) (`self.StaticMesh`))
  (`PrimitiveComponent.SetMaterial` (`self.StaticMesh`) 0 (`|GetArrayItem` _paints (`KismetMathLibrary.RandomIntegerInRange` 0 (- (`KismetArrayLibrary.Array_Length` _paints) 1))))
  (`/Game/Blueprints/ValetGameMode.RegisterNewCar` (cast `/Game/Blueprints/ValetGameMode` (`GameplayStatics.GetGameMode`) :!pure true) self))

(event `self.ReceiveUnpossessed`
  (params (OldController :type "Controller Object Reference"))
  (`AudioComponent.SetSound` (`self.CarSounds`) "/Game/Audio/EngineGasEnd.EngineGasEnd")
  (`AudioComponent.Play` (`self.CarSounds`) 0.0)
  (`AudioComponent.Play` (`self.CarSounds`) 0.0))

(event `self.ReceivePossessed`
  (params (NewController :type "Controller Object Reference"))
  (bind _carsounds (`self.CarSounds`))
  (cast `PlayerController` NewController
    (:`then`
      (`AudioComponent.SetSound` _carsounds "/Game/Audio/EngineStart.EngineStart")
      (`AudioComponent.Play` _carsounds 0.0)
      (`ActorComponent.Deactivate` (`self.FloatingPawnMovement`)))
    (:`CastFailed`
      (`ActorComponent.Activate` (`self.FloatingPawnMovement`) true))))

(event `InputAxis|Forward`
  (params (AxisValue :type "Float (single-precision)"))
  (bind _carsounds (`self.CarSounds`))
  ;[1 1 1] Movement
  (`PrimitiveComponent.AddForce` (`self.StaticMesh`) (* (* (`SceneComponent.GetForwardVector` (`self.Arrow`)) AxisValue) (`self.MovementForce`)) "None" false)
  (if (> AxisValue 0.0)
    (`/Engine/EditorBlueprintResources/StandardMacros.DoOnce` false :!label _label
      (:`Completed`
        (`AudioComponent.SetSound` _carsounds "/Game/Audio/EngineGasLoop_Cue.EngineGasLoop_Cue")
        (`AudioComponent.Play` _carsounds 0.0)))
    (else
      (goto _label :!via `Reset`))))

(event `self.ReceiveTick`
  (params (DeltaSeconds :type "Float (single-precision)"))
  ;[1 1 1] Tick Events
  (`self.Check If Moving`))

(event `InputAction|Interact`
  (params (Key :type "Key Structure"))
  (bind _staticmesh (`self.StaticMesh`))
  ;[1 1 1] Interaction
  (:`Pressed`
    (bind _returnvalue (`|SpawnActorFromClass` "/Game/Blueprints/ValetPawn.ValetPawn_C" (`KismetMathLibrary.MakeTransform` (+ (+ (`SceneComponent.K2_GetComponentLocation` _staticmesh) (* (`SceneComponent.GetRightVector` _staticmesh) -350.0)) (* (`SceneComponent.GetUpVector` _staticmesh) 50.0))) "AdjustIfPossibleButAlwaysSpawn" "OverrideRootScale" null null))
    (`/Engine/EditorBlueprintResources/StandardMacros.IsValid` _returnvalue
      (:`Is Valid`
        (`Controller.Possess` (`GameplayStatics.GetPlayerController` 0) _returnvalue)
        (`self.CarExited`)
        (if (`self.IsAbleToPark`)
          (if (not (`self.CarParked`))
            (`/Game/Blueprints/ValetGameMode.CarParked` (cast `/Game/Blueprints/ValetGameMode` (`GameplayStatics.GetGameMode`) :!pure true) self)))))))

(event `InputAxis|Left`
  (params (AxisValue :type "Float (single-precision)"))
  ;[1 1 1] Movement
  (bind _result (`/Engine/EditorBlueprintResources/StandardMacros.NegateFloat` AxisValue)
    (:`  `
      (if (not (`self.TurnLocked`))
        (`SceneComponent.K2_AddLocalRotation` (`self.StaticMesh`) (`KismetMathLibrary.MakeRotator` 0.0 0.0 (* (`self.RotationSpeed`) _result)) false false)))))

(event `InputAxis|Right`
  (params (AxisValue :type "Float (single-precision)"))
  ;[1 1 1] Movement
  (if (not (`self.TurnLocked`))
    (`SceneComponent.K2_AddLocalRotation` (`self.StaticMesh`) (`KismetMathLibrary.MakeRotator` 0.0 0.0 (* (`self.RotationSpeed`) AxisValue)) false false)))

(event `InputAxis|Backward`
  (params (AxisValue :type "Float (single-precision)"))
  ;[1 1 1] Movement
  (bind _result (`/Engine/EditorBlueprintResources/StandardMacros.NegateFloat` AxisValue)
    (:`  `
      (`PrimitiveComponent.AddForce` (`self.StaticMesh`) (* (* (`SceneComponent.GetForwardVector` (`self.Arrow`)) _result) (`self.MovementForce`)) "None" false))))

(event `self.StaticMesh.OnComponentBeginOverlap`
  (params (OverlappedComponent :type "PrimitiveComponent Object Reference") (OtherActor :type "Actor Object Reference") (OtherComp :type "PrimitiveComponent Object Reference") (OtherBodyIndex :type Integer) (bFromSweep :type Boolean) (SweepResult :type "HitResult Structure (by ref)"))
  (cast `/Game/Blueprints/PArkingZone` OtherActor)
  (set `self.IsAbleToPark` true))

(event `self.StaticMesh.OnComponentEndOverlap`
  (params (OverlappedComponent :type "PrimitiveComponent Object Reference") (OtherActor :type "Actor Object Reference") (OtherComp :type "PrimitiveComponent Object Reference") (OtherBodyIndex :type Integer))
  (cast `/Game/Blueprints/PArkingZone` OtherActor)
  (set `self.IsAbleToPark` false))

(event `self.CarSounds.OnAudioFinished`)

(fn `Check If Moving`
  (bind _returnvalue (`PrimitiveComponent.GetPhysicsLinearVelocity` (`self.StaticMesh`) "None"))
  (set `self.TurnLocked` (not (or (> (.x _returnvalue) 0.5) (< (.x _returnvalue) -0.5)))))

(fn `GetCarID`
  (returns (ID :type "Float (double-precision)"))
  (return (`self.CarID`)))

(fn `SetCarID`
  (params (ID :type "Float (double-precision)"))
  (set `self.CarID` ID))

(fn `UserConstructionScript`)