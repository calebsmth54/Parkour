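; Game mode for a valet game that gives cars random IDs and tracks the one to retrieve.
; RegisterNewCar sets a car's ID through CheckIDRandom, which recursively rerolls random floats already in SpawnedCarIDs and records new ones.
; CarParked flags the car pawn as parked and stores its ID in CarIDToRetrieve.
; GetCarByID is an empty stub, and BeginPlay and Tick are unused.
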(fn `CarParked`
  (params (CarPawn :type "/Game/Blueprints/CarPawn Object Reference"))
  (bind _id (`/Game/Blueprints/CarPawn.GetCarID` CarPawn))
  (set `self.CarIDToRetrieve` _id)
  (set `/Game/Blueprints/CarPawn.CarParked` true CarPawn))

(fn `CheckIDRandom`
  (params (ID :type "Float (double-precision)"))
  (returns (UniqueID :type "Float (double-precision)"))
  (if (`BlueprintSetLibrary.Set_Contains` (`self.SpawnedCarIDs`) ID)
    (bind _uniqueid (`self.CheckIDRandom` (`KismetMathLibrary.RandomFloat`)))
    (else
      (`BlueprintSetLibrary.Set_Add` (`self.SpawnedCarIDs`) ID)))
  (return _uniqueid))

(fn `GetCarByID`)

(fn `RegisterNewCar`
  (params (Car :type "/Game/Blueprints/CarPawn Object Reference"))
  (bind _uniqueid (`self.CheckIDRandom` (`KismetMathLibrary.RandomFloat`)))
  (`/Game/Blueprints/CarPawn.SetCarID` Car _uniqueid))

(fn `UserConstructionScript`)