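; ValetPawn is the player-controlled valet pawn that can take control of nearby cars.
; Axis inputs drive it by applying force to its static mesh along an arrow's forward vector and yawing the mesh to turn.
; Each tick, a short debug-drawn forward line trace stores any CarPawn hit as the possession target.
; Pressing Interact with a valid target possesses that car and destroys the valet.
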(event `InputAxis|Forward`
  (params (AxisValue :type "Float (single-precision)"))
  ;[1 1 1] Movement
  (`PrimitiveComponent.AddForce` (`self.StaticMesh`) (* (* (`SceneComponent.GetForwardVector` (`self.Arrow`)) AxisValue) (`self.MovementSpeed`)) "None" false))

(event `InputAction|Interact`
  (params (Key :type "Key Structure"))
  (bind _posessable (`self.Posessable`))
  ;[1 1 1] Interaction
  (:`Pressed`
    (if (`self.IsInteracting`)
      (`/Engine/EditorBlueprintResources/StandardMacros.IsValid` _posessable
        (:`Is Valid`
          (`Controller.Possess` (`GameplayStatics.GetPlayerController` 0) _posessable)
          (`self.K2_DestroyActor`))))))

(event `InputAxis|Left`
  (params (AxisValue :type "Float (single-precision)"))
  ;[1 1 1] Movement
  (bind _result (`/Engine/EditorBlueprintResources/StandardMacros.NegateFloat` AxisValue)
    (:`  `
      (`SceneComponent.K2_AddLocalRotation` (`self.StaticMesh`) (`KismetMathLibrary.MakeRotator` 0.0 0.0 (* (`self.RotationSpeed`) _result)) false false))))

(event `InputAxis|Right`
  (params (AxisValue :type "Float (single-precision)"))
  ;[1 1 1] Movement
  (`SceneComponent.K2_AddLocalRotation` (`self.StaticMesh`) (`KismetMathLibrary.MakeRotator` 0.0 0.0 (* (`self.RotationSpeed`) AxisValue)) false false))

(event `self.ReceiveTick`
  (params (DeltaSeconds :type "Float (single-precision)"))
  (bind _staticmesh (`self.StaticMesh`))
  (bind _returnvalue (`SceneComponent.K2_GetComponentLocation` _staticmesh))
  ;[1 1 1] Interaction Raycast
  (bind (_outhit _returnvalue_2) (`KismetSystemLibrary.LineTraceSingle` :`Start` _returnvalue :`End` (+ _returnvalue (* (`SceneComponent.GetForwardVector` _staticmesh) 200.0)) :`TraceChannel` (enumliteral `ETraceTypeQuery` "TraceTypeQuery1") :`DrawDebugType` "ForOneFrame"))
  (if _returnvalue_2
    (bind _ascar_pawn (cast `/Game/Blueprints/CarPawn` (`.HitActor` (`GameplayStatics.BreakHitResult` _outhit)))
      (:`then`
        (set `self.IsInteracting` true)
        (set `self.Posessable` _ascar_pawn))
      (:`CastFailed`
        (set `self.IsInteracting` false :!label _label)
        (set `self.Posessable` null)))
    (else
      (goto _label))))

(event `InputAxis|Backward`
  (params (AxisValue :type "Float (single-precision)"))
  ;[1 1 1] Movement
  (bind _result (`/Engine/EditorBlueprintResources/StandardMacros.NegateFloat` AxisValue)
    (:`  `
      (`PrimitiveComponent.AddForce` (`self.StaticMesh`) (* (* (`SceneComponent.GetForwardVector` (`self.Arrow`)) _result) (`self.MovementSpeed`)) "None" false))))

(fn `UserConstructionScript`)