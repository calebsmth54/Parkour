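; CarSpawner is an actor that periodically spawns AI-driven cars and sends them toward a drop-off point.
; A looping two-second timer started on BeginPlay calls SpawnCar, which spawns a CarPawn with the AIDropOffCar behavior tree at the SpawnStart transform.
; Each car's controller then gets a simple move order to the DropOff location.
; A blackboard write that would pass DropOff to the tree is left unconnected.
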(event `self.ReceiveBeginPlay`
  (`KismetSystemLibrary.K2_SetTimerDelegate` (delegate `CustomEvent_0`) 2.0 true))

(event `CustomEvent_0`
  (`self.SpawnCar`))

(fn `SpawnCar`
  (locals (Key_DropOffpoint :type String :default "DropOffZone"))
  (bind _spawnstart (`self.SpawnStart`))
  (bind _returnvalue (`AIBlueprintHelperLibrary.SpawnAIFromClass` "/Game/Blueprints/CarPawn.CarPawn_C" "/Game/AI/AIDropOffCar.AIDropOffCar" (`SceneComponent.K2_GetComponentLocation` _spawnstart) (`SceneComponent.K2_GetComponentRotation` _spawnstart) true))
  (`AIBlueprintHelperLibrary.SimpleMoveToLocation` (`AIBlueprintHelperLibrary.GetAIController` _returnvalue) (`SceneComponent.K2_GetComponentLocation` (`self.DropOff`))))

(fn `UserConstructionScript`)